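; BP_Pistol is a pistol weapon that fires BP_Bullet projectiles.
; On Fire it spawns the bullet at the mesh's Ammo socket, nudged by a camera-rotated ProjectileOffset and aimed along the player camera's rotation.
; It then plays a firing sound at that point and a one-shot fire animation on the skeletal mesh.
; Camera manager and socket lookups avoid hard references and model-specific logic.
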(event EventFire
  (params (Gun :type BP%20Weapon%20Object%20Reference))
  (bind _returnvalue (Game|GetPlayerCameraManager 0))
  (bind _projectileoffset (Variables|Default|GetProjectileOffset))
  (bind _skeletalmesh (Variables|Default|GetSkeletalMesh))
  (bind _returnvalue_2 (Camera|GetCameraRotation _returnvalue))
  (bind _returnvalue_3 (Transformation|GetSocketLocation _skeletalmesh "Ammo"))
  (bind _returnvalue_4 (Math|Vector|RotateVector _projectileoffset _returnvalue_2))
  (bind _returnvalue_5 (+ _returnvalue_3 _returnvalue_4))
  (Game|SpawnActorfromClass "/Game/_MyBlueprints/Weapons/BP_Ammo/BP_Bullet.BP_Bullet_C" (Math|Transform|MakeTransform _returnvalue_5 _returnvalue_2) "Undefined" 0 false "/Game/MilitaryWeapDark/FX/P_Grenade_Explosion_01.P_Grenade_Explosion_01" false 0 0)
  (Audio|PlaySoundatLocation 0 _returnvalue_5 "0, 0, 0" 1.0 1.0 0.0 0 0 0 0) ; Play firing sound
  (Components|Animation|PlayAnimation (Variables|Default|GetSkeletalMesh) "/Game/MilitaryWeapSilver/Weapons/Animations/Fire_Pistol_W.Fire_Pistol_W" false))

(fn ConstructionScript
  (|CallParentFunction))