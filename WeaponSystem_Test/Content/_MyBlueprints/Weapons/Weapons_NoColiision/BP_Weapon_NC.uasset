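; Weapon actor, in the no-collision weapons folder, that fires projectiles and can be dropped.
; Fire branches on authority: the server calls replicated Multi events for shot and sound, while remotes run both locally.
; Shoot spawns AmmoType at an offset muzzle socket and always plays the rocket launcher fire animation.
; Drop enables mesh physics, then destroys the weapon after OngroundDuration.
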(event Custom|ProjSound_Multi
  ;[1 1 1] Replicated event to fire projectile on server
  (CallFunction|PlaySound)
  (Development|PrintString "Server Sound"))

(event Custom|Fire_Multi
  ;[1 1 1] Replicated event to fire projectile on server
  (CallFunction|Shoot)
  (Development|PrintString "Server Fire"))

(event EventDrop
  (params (weapon :type BP%20Weapon%20NC%20Object%20Reference))
  ;[1 1 1] Enables physics for weapon to fall to ground when dropped. After delay physics are disable and the actor is destroyed
  (Development|PrintString "drop")
  (Physics|SetSimulatePhysics (Variables|Default|GetSkeletalMesh) true)
  (Utilities|FlowControl|Delay (Variables|Default|GetOngroundDuration))
  (Physics|SetSimulatePhysics (Variables|Default|GetSkeletalMesh) false)
  (Actor|DestroyActor))

(event EventFire
  ;[1 1 1] Interface action to all fire action from character BP
  (Networking|SwitchHasAuthority
    (:Authority
      (CallFunction|FireMulti)
      (CallFunction|ProjSoundMulti))
    (:Remote
      (CallFunction|Shoot)
      (CallFunction|PlaySound))))

(fn ConstructionScript
  (Physics|SetSimulatePhysics (Variables|Default|GetSkeletalMesh) false))

(fn Shoot
  (bind _skeletalmesh (Variables|Default|GetSkeletalMesh))
  (bind _in_socket_name (Variables|Default|GetIn%20Socket%20Name))
  (bind _output_get (Variables|Default|SetProjectileLocation (+ (Transformation|GetSocketLocation _skeletalmesh _in_socket_name) (Variables|Default|GetProjectileOffset))))
  (Game|SpawnActorfromClass (Variables|Default|GetAmmoType) (Math|Transform|MakeTransform _output_get (Transformation|GetSocketRotation _skeletalmesh _in_socket_name)) "AdjustIfPossibleButAlwaysSpawn" 0 false 0 false 0 0 "None" 0)
  (Components|Animation|PlayAnimation (Variables|Default|GetSkeletalMesh) "/Game/MilitaryWeapSilver/Weapons/Animations/Fire_RocketLauncher_W.Fire_RocketLauncher_W" false))

(fn PlaySound
  (Audio|PlaySoundatLocation (Variables|Default|GetFiringSound) (Variables|Default|GetProjectileLocation) "0, 0, 0" 1.0 1.0 0.0 0 0 0 0))