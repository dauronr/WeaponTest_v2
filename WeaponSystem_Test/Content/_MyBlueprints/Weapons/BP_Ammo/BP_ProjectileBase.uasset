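; BP_ProjectileBase is a weapon projectile base with configurable trail, explosion and impact sound.
; BeginPlay optionally attaches a trail emitter to the projectile mesh.
; On hit, it triggers the optional explosion emitter through Boom, pushes the struck component with a velocity-scaled impulse, fires a radial force, plays the sound and destroys itself.
; The physics-simulation check calls the explosion on both branches.
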(event Custom|Explosion
  ;[1 1 1] Calls Boom function for explosion
  (CallFunction|Boom))

(event EventBeginPlay
  (bind _projectilemesh (Variables|Default|GetProjectileMesh))
  ;[1 1 1] Creats emitter for trail smoke
  (if (Variables|Default|GetNeedsTrailEmitter?)
    (Effects|SpawnEmitterAttached (Variables|Default|GetTrail%20Emitter) _projectilemesh (Variables|Default|GetAttach%20Point%20Name) (Variables|/Script/Engine.SceneComponent|GetRelativeLocation _projectilemesh) (Variables|/Script/Engine.SceneComponent|GetRelativeRotation _projectilemesh))))

(event Collision|EventHit
  (params (MyComp :type Primitive%20Component%20Object%20Reference) (Other :type Actor%20Object%20Reference) (OtherComp :type Primitive%20Component%20Object%20Reference) (bSelfMoved :type Boolean) (HitLocation :type Vector :default "0, 0, 0") (HitNormal :type Vector :default "0, 0, 0") (NormalImpulse :type Vector :default "0, 0, 0") (Hit :type Hit%20Result%20Structure%20%28by%20ref%29))
  (bind _returnvalue (Transformation|GetActorLocation))
  ;[1 1 1] On hit checks for objects simulating physics, adds force based on configurable projectile speed. Calls customer event for explosion and destroys actor acter
  (if (Physics|IsSimulatingPhysics OtherComp "None")
    (CallFunction|Explosion)
    (else
      (CallFunction|Explosion)))
  (Physics|AddImpulseatLocation OtherComp (* (Transformation|GetVelocity) 1e+02) _returnvalue "None")
  (Class|RadialForceComponent|FireImpulse (Variables|Default|GetRadialForce))
  (Audio|PlaySoundatLocation (Variables|Default|GetImpact%20Sound) _returnvalue "0, 0, 0" 1.0 1.0 0.0 0 0 0 0)
  (Actor|DestroyActor))

(fn ConstructionScript)

(fn Boom
  ;[1 1 1] Emitter event. Emitter variable exposed for easy changing in editor
  ; Checks if explosion is need for specific projectile type
  (if (Variables|Default|GetNeedExplosion?)
    (Effects|SpawnEmitteratLocation (Variables|Default|GetExplosion%20Emitter) (Transformation|GetActorLocation) (Transformation|GetActorRotation))))