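; BP_Rocket_Base is a base rocket projectile that explodes on hit and pushes objects with physics forces.
; BeginPlay attaches a smoke trail emitter to the rocket mesh.
; On hit, both branches of a physics-simulation check spawn the configurable explosion emitter, then a velocity-scaled impulse hits the struck component, RadialForce fires and the actor destroys itself.
; The file applies no damage, only effects and impulses.
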(event Custom|Explosion
  ;[1 1 1] Emitter event. Emitter variable exposed for easy changing in editor
  (Effects|SpawnEmitteratLocation (Variables|Default|GetEmitter) (Transformation|GetActorLocation) (Transformation|GetActorRotation)))

(event EventBeginPlay
  (bind _grenadelaunchera_ammo (Variables|Default|GetGrenadeLauncherA_Ammo))
  ;[1 1 1] Creats emitter for trail smoke
  (Effects|SpawnEmitterAttached "/Game/MilitaryWeapDark/FX/P_RocketLauncher_Trail_01.P_RocketLauncher_Trail_01" _grenadelaunchera_ammo "None" (Variables|/Script/Engine.SceneComponent|GetRelativeLocation _grenadelaunchera_ammo) (Variables|/Script/Engine.SceneComponent|GetRelativeRotation _grenadelaunchera_ammo)))

(event Collision|EventHit
  (params (MyComp :type Primitive%20Component%20Object%20Reference) (Other :type Actor%20Object%20Reference) (OtherComp :type Primitive%20Component%20Object%20Reference) (bSelfMoved :type Boolean) (HitLocation :type Vector :default "0, 0, 0") (HitNormal :type Vector :default "0, 0, 0") (NormalImpulse :type Vector :default "0, 0, 0") (Hit :type Hit%20Result%20Structure%20%28by%20ref%29))
  ;[1 1 1] On hit checks for objects simulating physics, adds force based on configurable projectile speed. Calls customer event for explosion and destroys actor acter
  (if (Physics|IsSimulatingPhysics OtherComp "None")
    (CallFunction|Explosion)
    (else
      (CallFunction|Explosion)))
  (Physics|AddImpulseatLocation OtherComp (* (Transformation|GetVelocity) 1e+02) (Transformation|GetActorLocation) "None")
  (Class|RadialForceComponent|FireImpulse (Variables|Default|GetRadialForce))
  (Actor|DestroyActor))

(fn ConstructionScript)